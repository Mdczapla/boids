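; BP_Predator is a boids-style predator actor that chases the nearest BP_Boid.
; Each tick, CalculateChase scans all boids for the closest and returns a seek steering vector: desired velocity at MaxSpeed minus current Vel.
; That vector, scaled by ChaseWeight, is added to Vel, which is clamped to MaxSpeed.
; Vel is applied as an unswept local-space offset each frame, without delta-time scaling.
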(event EventBeginPlay)

(event Collision|EventActorBeginOverlap
  (params (OtherActor :type Actor%20Object%20Reference)))

(event EventTick
  (params (DeltaSeconds :type Float%20%28single-precision%29))
  (bind _force (CallFunction|CalculateChase))
  (bind _output_get (Variables|Default|SetVel (+ (* _force (Variables|Default|GetChaseWeight)) (stale _output_get))))
  (bind _output_get_2 (Variables|Default|SetVel (Math|Vector|VectorClampSizeMax (Variables|Default|GetVel) (Variables|Default|GetMaxSpeed))))
  (Transformation|AddActorLocalOffset _output_get_2 false false))

(fn ConstructionScript)

(fn CalculateChase
  (bind _returnvalue (Transformation|GetActorLocation))
  (bind _outactors (Actor|GetAllActorsOfClass "/Game/Blueprints/BP_Boid.BP_Boid_C"))
  (LocalVariables|SetMinDistance (Math|Vector|Distance(Vector) (Transformation|GetActorLocation (Utilities|Array|Get(acopy) _outactors)) _returnvalue))
  (LocalVariables|SetNearestVictim (Utilities|Array|Get(acopy) _outactors))
  (for _array_element _outactors
    (if (< (Math|Vector|Distance(Vector) (Transformation|GetActorLocation _array_element) _returnvalue) (LocalVariables|GetMinDistance))
      (LocalVariables|SetMinDistance (Math|Vector|Distance(Vector) (Transformation|GetActorLocation _array_element) _returnvalue))
      (LocalVariables|SetNearestVictim _array_element)))
  (LocalVariables|SetTemp (- (* (Math|Vector|Normalize (- (Transformation|GetActorLocation (LocalVariables|GetNearestVictim)) _returnvalue)) (Variables|Default|GetMaxSpeed)) (Variables|Default|GetVel)))
  (return (LocalVariables|GetTemp)))