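; Flocking agent actor that starts with a random XY velocity and steers among other boids while fleeing BP_Predator actors.
; Each Tick adds weighted separation, alignment and cohesion from Sphere overlaps, plus avoidance from a distance check over all predators, to its velocity.
; Velocity is clamped to MaxSpeed, scaled by FleingModifier when fleeing, then applied as an unswept world offset without delta-time scaling or rotation.
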(event EventBeginPlay
  (bind _returnvalue (Math|Random|RandomFloatinRange -1.0 1.0))
  (Math|Random|SetRandomStreamSeed (Variables|Default|GetStream) 0)
  (Variables|Default|SetVel (* (Math|Vector|Normalize (Math|Vector|MakeVector _returnvalue _returnvalue 0.0)) (Variables|Default|GetMaxSpeed))))

(event Collision|EventActorBeginOverlap
  (params (OtherActor :type Actor%20Object%20Reference)))

(event EventTick
  (params (DeltaSeconds :type Float%20%28single-precision%29))
  (Variables|Default|SetSep "0, 0, 0")
  (Variables|Default|SetAli "0, 0, 0")
  (Variables|Default|SetCoh "0, 0, 0")
  (Variables|Default|SetAvo "0, 0, 0")
  (bind _force (CallFunction|CalculateSeparation))
  (if (Math|Vector|VectorIsNearlyZero _force 0.01)
    _
    (else
      (Variables|Default|SetSep (* _force (Variables|Default|GetSeparationWeight)))))
  (bind _force_2 (CallFunction|CalculateAlignment))
  (if (Math|Vector|VectorIsNearlyZero _force_2 0.01)
    _
    (else
      (Variables|Default|SetAli (* _force_2 (Variables|Default|GetAlignmentWeight)))))
  (bind _force_3 (CallFunction|CalculateCohesion))
  (if (Math|Vector|VectorIsNearlyZero _force_3 0.01)
    _
    (else
      (Variables|Default|SetCoh (* _force_3 (Variables|Default|GetCohesionWeight)))))
  (bind _force_4 (CallFunction|CalculateAvoidPredator))
  (if (Math|Vector|VectorIsNearlyZero _force_4 0.01)
    _
    (else
      (Variables|Default|SetAvo (* _force_4 (Variables|Default|GetAvoidanceWeight)))))
  (bind _output_get (Variables|Default|SetVel (+ (+ (Variables|Default|GetSep) (Variables|Default|GetAli) (Variables|Default|GetCoh) (Variables|Default|GetAvo)) (stale _output_get))))
  (Variables|Default|SetVel (Math|Vector|VectorClampSizeMax (Variables|Default|GetVel) (Variables|Default|GetMaxSpeed)))
  (if (Math|Vector|VectorIsNearlyZero (Variables|Default|GetAvo) 0.001)
    _
    (else
      (bind _output_get_2 (Variables|Default|SetVel (* (stale _output_get_2) (Variables|Default|GetFleingModifier))))))
  (Transformation|AddActorWorldOffset (Variables|Default|GetVel)))

(fn ConstructionScript)

(fn CalculateAvoidPredator
  (bind _returnvalue (Transformation|GetActorLocation))
  (bind _output_get (LocalVariables|SetNumOfNearby 0))
  (bind _outactors (Actor|GetAllActorsOfClass "/Game/Blueprints/BP_Predator.BP_Predator_C"))
  (for _array_element _outactors
    (if (< (Math|Vector|Distance(Vector) (Transformation|GetActorLocation _array_element) _returnvalue) (Variables|Default|GetPredatorDetectionRadius))
      (Math|Integer|IncrementInt _output_get
        (:%20%20
          (bind _output_get_2 (LocalVariables|SetAvoidForce (+ (stale _output_get_2) (/ (- _returnvalue (Transformation|GetActorLocation _array_element)) (Math|Vector|Distance(Vector) (Transformation|GetActorLocation _array_element) _returnvalue)))))))))
  (if (> (LocalVariables|GetNumOfNearby) 0)
    (LocalVariables|SetTemp (* (Math|Vector|Normalize (/ (LocalVariables|GetAvoidForce) (LocalVariables|GetNumOfNearby))) (Variables|Default|GetMaxSpeed)))
    (else
      (LocalVariables|SetTemp "0, 0, 0")))
  (return (LocalVariables|GetTemp)))

(fn CalculateSeparation
  (bind _returnvalue (Transformation|GetActorLocation))
  (bind _output_get (LocalVariables|SetNumOfNearby 0))
  (for _array_element (Collision|GetOverlappingActors (Variables|Default|GetSphere) "BP_Boid_C" :!class /Script/Engine.PrimitiveComponent)
    (Math|Integer|IncrementInt _output_get
      (:%20%20
        (bind _output_get_2 (LocalVariables|SetSeparationForce (+ (stale _output_get_2) (/ (- _returnvalue (Transformation|GetActorLocation _array_element)) (Math|Vector|Distance(Vector) (Transformation|GetActorLocation _array_element) _returnvalue))))))))
  (if (> (LocalVariables|GetNumOfNearby) 0)
    (LocalVariables|SetTemp (- (* (Math|Vector|Normalize (/ (LocalVariables|GetSeparationForce) (LocalVariables|GetNumOfNearby))) (Variables|Default|GetMaxSpeed)) (Variables|Default|GetVel)))
    (else
      (LocalVariables|SetTemp "0, 0, 0")))
  (return (LocalVariables|GetTemp)))

(fn CalculateAlignment
  (bind _output_get (LocalVariables|SetNumOfNearby 0))
  (for _array_element (Collision|GetOverlappingActors (Variables|Default|GetSphere) "BP_Boid_C" :!class /Script/Engine.PrimitiveComponent)
    (Math|Integer|IncrementInt _output_get
      (:%20%20
        (bind _asbp_boid (Utilities|Casting|CastToBP_Boid _array_element))
        (bind _output_get_2 (LocalVariables|SetAverageVelocity (+ (stale _output_get_2) (Variables|BP_Boid_C|GetVel _asbp_boid)))))))
  (if (> (LocalVariables|GetNumOfNearby) 0)
    (LocalVariables|SetTemp (- (* (Math|Vector|Normalize (/ (LocalVariables|GetAverageVelocity) (LocalVariables|GetNumOfNearby))) (Variables|Default|GetMaxSpeed)) (Variables|Default|GetVel)))
    (else
      (LocalVariables|SetTemp "0, 0, 0")))
  (return (LocalVariables|GetTemp)))

(fn CalculateCohesion
  (bind _output_get (LocalVariables|SetNumOfNearby 0))
  (for _array_element (Collision|GetOverlappingActors (Variables|Default|GetSphere) "BP_Boid_C" :!class /Script/Engine.PrimitiveComponent)
    (Math|Integer|IncrementInt _output_get
      (:%20%20
        (bind _output_get_2 (LocalVariables|SetCenterOfMass (+ (stale _output_get_2) (Transformation|GetActorLocation _array_element)))))))
  (if (> (LocalVariables|GetNumOfNearby) 0)
    (LocalVariables|SetTemp (- (* (Math|Vector|Normalize (- (/ (LocalVariables|GetCenterOfMass) (LocalVariables|GetNumOfNearby)) (Transformation|GetActorLocation))) (Variables|Default|GetMaxSpeed)) (Variables|Default|GetVel)))
    (else
      (LocalVariables|SetTemp "0, 0, 0")))
  (return (LocalVariables|GetTemp)))