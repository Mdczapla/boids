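; BP_Setup is a spawner actor that populates a boid flocking scene with prey and predators when play begins.
; BeginPlay runs two loops, spawning BP_Boid for the victim count and BP_Predator for the predator count.
; Each spawn location is a random point in a box centered on the actor, with X and Y half-extents taken from Area.
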(event EventBeginPlay
  (bind _area (Variables|Default|GetArea))
  (bind _area_2 (Variables|Default|GetArea))
  (for _index (range 0 (- (Variables|Default|GetNumOfVictims) 1))
    (Game|SpawnActorfromClass "/Game/Blueprints/BP_Boid.BP_Boid_C" (Math|Transform|MakeTransform (Math|Random|RandomPointinBoundingBox (Transformation|GetActorLocation) (Math|Vector|MakeVector (.x _area_2) (.y _area_2) 0.0)) "0, 0, 0" "1.000000,1.000000,1.000000") "Undefined" "MultiplyWithRoot" 0 0))
  (for _index_2 (range 0 (- (Variables|Default|GetNumOfPredators) 1))
    (Game|SpawnActorfromClass "/Game/Blueprints/BP_Predator.BP_Predator_C" (Math|Transform|MakeTransform (Math|Random|RandomPointinBoundingBox (Transformation|GetActorLocation) (Math|Vector|MakeVector (.x _area) (.y _area) 0.0)) "0, 0, 0" "1.000000,1.000000,1.000000") "Undefined" "MultiplyWithRoot" 0 0)))

(event Collision|EventActorBeginOverlap
  (params (OtherActor :type Actor%20Object%20Reference)))

(event EventTick
  (params (DeltaSeconds :type Float%20%28single-precision%29)))

(fn ConstructionScript)